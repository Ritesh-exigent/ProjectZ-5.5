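; BP_Bullet_P is a bullet projectile actor that flies straight along its forward vector.
; Tick offsets it by Speed scaled by delta time, without sweep, and accumulates Lifetime, destroying it on reaching MaxLifetime.
; Any actor overlap prints a debug message and destroys the bullet, with no damage applied in this graph.
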(event `self.ReceiveActorBeginOverlap`
  (params (OtherActor :type "Actor Object Reference"))
  (`KismetSystemLibrary.PrintString` "Bullet overlapped")
  (`self.K2_DestroyActor`))

(event `self.ReceiveTick`
  (params (DeltaSeconds :type "Float (single-precision)"))
  (`self.K2_AddActorWorldOffset` (* (`self.GetActorForwardVector`) DeltaSeconds (`self.Speed`)))
  (bind _output_get (set `self.Lifetime` (+ (`self.Lifetime`) DeltaSeconds)))
  (if (>= _output_get (`self.MaxLifetime`))
    (`self.K2_DestroyActor`)))

(fn `UserConstructionScript`)