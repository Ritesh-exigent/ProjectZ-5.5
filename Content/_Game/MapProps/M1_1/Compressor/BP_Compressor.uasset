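; BP_Compressor is an interactable compressor map prop with an animated door on its Cover mesh.
; BeginPlay plays the door close animation, and InteractBP calls Switch, which only plays the open animation because its open/close FlipFlop is disconnected.
; The Box overlap casts to ZEnemy but does nothing further, as the OnDeath kill call is also disconnected.
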(event `self.ReceiveBeginPlay`
  (`SkeletalMeshComponent.PlayAnimation` (`self.Cover`) "/Game/_Game/MapProps/M1_1/Compressor/Door/Anim/AS_Compressor_Door_Close.AS_Compressor_Door_Close" false))

(event `InteractionInterface.Interact_BP`
  (params (InPlayer :type "SPlayer Object Reference"))
  (`self.Switch`))

(event `self.Box.OnComponentBeginOverlap`
  (params (OverlappedComponent :type "PrimitiveComponent Object Reference") (OtherActor :type "Actor Object Reference") (OtherComp :type "PrimitiveComponent Object Reference") (OtherBodyIndex :type Integer) (bFromSweep :type Boolean) (SweepResult :type "HitResult Structure (by ref)"))
  (bind _aszenemy (cast `ZEnemy` OtherActor)))

(fn `Switch`
  (`SkeletalMeshComponent.PlayAnimation` (`self.Cover`) "/Game/_Game/MapProps/M1_1/Compressor/Door/Anim/AS_Compressor_Door_Open.AS_Compressor_Door_Open" false))

(fn `UserConstructionScript`)