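; BP_ELight is an electric room prop light that randomly flickers its RectLight when EnableFlicker is set.
; Each Tick outside cooldown rolls against FlickerProbablity to start a burst, which toggles intensity between off and full after each FlickerDelay.
; Bursts end after MaxFlickTime, leaving the last intensity in place, then wait CooldownTime.
; Both waits use Delay nodes directly on Tick.
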(event `self.ReceiveTick`
  (params (DeltaSeconds :type "Float (single-precision)"))
  (if (`self.bEnableFlicker`)
    (if (`self.bCooldown`)
      (`KismetSystemLibrary.Delay` (`self.CooldownTime`))
      (set `self.bCooldown` false)
      (else
        (`|ExecutionSequence`
          (:`then_0`
            (if (and (not (`self.bFlicker`)) (<= (`KismetMathLibrary.RandomFloatInRange` 0.0 1.0) (`self.FlickerProbablity`)))
              (set `self.bFlicker` true)))
          (:`then_1`
            (if (`self.bFlicker`)
              (bind _output_get (set `self.CurrentFlickTime` (+ (`self.CurrentFlickTime`) DeltaSeconds)))
              (if (>= _output_get (`self.MaxFlickTime`))
                (set `self.bFlicker` false)
                (set `self.CurrentFlickTime` 0.0)
                (set `self.bCooldown` true)
                (else
                  (`KismetSystemLibrary.Delay` (`self.FlickerDelay`))
                  (bind _output_get_2 (set `self.Switch` (- 1.0 (`self.Switch`))))
                  (`LightComponent.SetIntensity` (`self.RectLight`) (* _output_get_2 5000.0)))))))))))

(fn `UserConstructionScript`)