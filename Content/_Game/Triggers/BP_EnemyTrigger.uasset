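; BP_EnemyTrigger is a one-shot trigger volume that starts enemy spawning when something begins overlapping its box.
; The overlap gets the enemy manager from BP_ZGameMode, falling back to BP_TestingGameMode, and calls DispatchSpawn on it.
; It then prints a debug message, sets AlreadyTriggered and destroys itself, with no filter on which actor overlaps.
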(event `self.Box.OnComponentBeginOverlap`
  (params (OverlappedComponent :type "PrimitiveComponent Object Reference") (OtherActor :type "Actor Object Reference") (OtherComp :type "PrimitiveComponent Object Reference") (OtherBodyIndex :type Integer) (bFromSweep :type Boolean) (SweepResult :type "HitResult Structure (by ref)"))
  (bind _returnvalue (`GameplayStatics.GetGameMode`))
  (if (not (`self.bAlreadyTriggered`))
    (bind _asbp_zgame_mode (cast `/Game/_Game/GameModes/BP_ZGameMode` _returnvalue)
      (:`then`
        (bind _returnvalue_2 (`ZGameMode.GetEnemyManager` _asbp_zgame_mode))
        (`ZEnemyManager.DispatchSpawn` _returnvalue_2))
      (:`CastFailed`
        (bind _asbp_testing_game_mode (cast `/Game/_Game/GameTesting/BP_TestingGameMode` _returnvalue))
        (bind _returnvalue_3 (`ZGameMode.GetEnemyManager` _asbp_testing_game_mode))
        (`ZEnemyManager.DispatchSpawn` _returnvalue_3)))
    (`KismetSystemLibrary.PrintString` "Enemy Triggered")
    (set `self.bAlreadyTriggered` true)
    (`self.K2_DestroyActor`)))

(fn `UserConstructionScript`)