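; BP_TestPlayer1 is a test player Blueprint that adds flashlight and weapon controls.
; Debug key X flip-flops the SpotLight intensity on and off, and debug key Q equips the next weapon through WComp.
; The IA_Reload Enhanced Input action calls reload on the same weapon component.
; Unconnected leftover logic would show the WBP_Story widget and initialize enemies through the BP_ZGameMode enemy manager, but it never runs.
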(event Input|EnhancedActionEvents|EnhancedInputActionIA_Reload
  (params (ActionValue :type Boolean) (ElapsedSeconds :type Float%20%28double-precision%29) (TriggeredSeconds :type Float%20%28double-precision%29) (InputAction :type Input%20Action%20Object%20Reference :default "/Game/_Game/Characters/Player/Input/Actions/IA_Reload.IA_Reload"))
  (Class|WeaponComponent|ReloadWeapon (Variables|Default|GetWComp)))

(event EventBeginPlay)

(event Collision|EventActorBeginOverlap
  (params (OtherActor :type Actor%20Object%20Reference)))

(event EventTick
  (params (DeltaSeconds :type Float%20%28single-precision%29)))

(event Input|KeyboardEvents|DebugKeyZ
  (params (Key :type Key%20Structure :default "None") (ActionValue :type Input%20Action%20Value%20Structure)))

(event Input|KeyboardEvents|DebugKeyQ
  (params (Key :type Key%20Structure :default "None") (ActionValue :type Input%20Action%20Value%20Structure))
  (bind _wcomp (Variables|Default|GetWComp))
  (:Pressed
    (Class|WeaponComponent|EquipWeapon _wcomp (Class|WeaponComponent|GetNextWeaponIndex _wcomp))))

(event Input|KeyboardEvents|DebugKeyX
  (params (Key :type Key%20Structure :default "None") (ActionValue :type Input%20Action%20Value%20Structure))
  (bind _spotlight (Variables|Default|GetSpotLight))
  (:Pressed
    (Utilities|FlowControl|FlipFlop
      (:A
        (Rendering|Components|Light|SetIntensity _spotlight 5e+03))
      (:B
        (Rendering|Components|Light|SetIntensity _spotlight 0.0)))))

(fn ConstructionScript)