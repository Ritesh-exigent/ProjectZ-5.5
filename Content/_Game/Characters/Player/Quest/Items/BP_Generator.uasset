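; BP_Generator is an interactable quest item that triggers the crane and belt overload and then the boss encounter.
; Interacting updates the current quest on BP_ZGameState, waits briefly, then calls MC_StartOverload.
; That event sets overload on the linked crane and, after a delay, starts the belt's overload.
; The interaction then finds BP_Boss in the level and initializes it after a further delay.
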(event `InteractionInterface.Interact_BP`
  (params (InPlayer :type "SPlayer Object Reference"))
  (bind _asbp_zgame_state (cast `/Game/_Game/Characters/Player/BP_ZGameState` (`GameplayStatics.GetGameState`)))
  (`ZGameState.UpdateCurrentQuest` _asbp_zgame_state)
  (`KismetSystemLibrary.Delay` 2.0)
  (`self.MC_StartOverload`)
  (bind _returnvalue (`GameplayStatics.GetActorOfClass` "/Game/_Game/Characters/AI/Enemies/BP/BP_Boss.BP_Boss_C"))
  (`KismetSystemLibrary.Delay` 5.0)
  (`ZEnemy.Init` _returnvalue))

(event `MC_StartOverload`
  (`Crane.SetOverload` (`self.BP_Crane`) true)
  (`KismetSystemLibrary.Delay` 2.0)
  (`/Game/_Game/MapProps/M1_1/Belt/BP_ConveyorBelt.StartOverload` (`self.BP_Belt`)))

(fn `UserConstructionScript`)