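; BP_CraneControl is an interactable that lets a player take control of the crane.
; On BeginPlay it finds and caches the BP_Crane in the level.
; On interaction, if the crane is neither in use nor overloaded, it has the player's ZPlayerController switch pawn to the crane; otherwise it only prints a debug message.
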(event `self.ReceiveBeginPlay`
  (bind _returnvalue (`GameplayStatics.GetActorOfClass` "/Game/_Game/MapProps/M1_1/Crane/BP_Crane.BP_Crane_C"))
  (set `self.Crane` _returnvalue))

(event `InteractionInterface.Interact_BP`
  (params (InPlayer :type "SPlayer Object Reference"))
  (bind _crane (`self.Crane`))
  (bind _returnvalue (`Crane.IsInUse` _crane))
  (`KismetSystemLibrary.PrintString` (`KismetStringLibrary.Conv_BoolToString` _returnvalue))
  (if (and (not _returnvalue) (not (`Crane.IsOverloaded` _crane)))
    (bind _aszplayer_controller (cast `ZPlayerController` (`Pawn.GetController` InPlayer)))
    (`ZPlayerController.SwitchPawn` _aszplayer_controller _crane)
    (else
      (`KismetSystemLibrary.PrintString` "Crane already in use"))))

(fn `UserConstructionScript`)