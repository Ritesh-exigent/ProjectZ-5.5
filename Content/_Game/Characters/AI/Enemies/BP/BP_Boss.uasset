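; BP_Boss is a boss enemy Blueprint that keeps a health bar widget in sync with its health.
; On BeginPlay it casts the Widget component's widget to WBP_HealthBar and caches the reference.
; Each Tick it sets the bar's percent from HDComp's current health divided by max health, polling rather than reacting to health change events.
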(event `self.ReceiveBeginPlay`
  (bind _widget (`self.Widget`))
  (`/Engine/EditorBlueprintResources/StandardMacros.IsValid` _widget
    (:`Is Valid`
      (bind _aswbp_health_bar (cast `/Game/_Game/Characters/AI/UI/WBP_HealthBar` (`WidgetComponent.GetWidget` _widget)))
      (set `self.HealthBar` _aswbp_health_bar))))

(event `self.ReceiveTick`
  (params (DeltaSeconds :type "Float (single-precision)"))
  (bind _healthbar (`self.HealthBar`))
  (bind _hdcomp (`self.HDComp`))
  (`/Engine/EditorBlueprintResources/StandardMacros.IsValid` _healthbar
    (:`Is Valid`
      (`ProgressBar.SetPercent` (`/Game/_Game/Characters/AI/UI/WBP_HealthBar.HealthBar` _healthbar) (/ (`HDComponent.GetHealth` _hdcomp) (`HDComponent.GetMaxHealth` _hdcomp))))))

(fn `UserConstructionScript`)